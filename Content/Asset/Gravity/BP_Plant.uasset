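; BP_Plant is a gravity source actor that pulls overlapping characters toward its center.
; On begin overlap, it sets the Character Movement gravity direction once, pointing from the character to the actor's location.
; For a BP_GravityCharacter, it also stores the overlapping actor, which is that character itself, in AActor.
; End overlap clears that reference but leaves the gravity direction unchanged.
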(event `self.ReceiveActorBeginOverlap`
  (params (OtherActor :type "Actor Object Reference"))
  (bind `_as캐릭터` (cast `Character` OtherActor))
  (`CharacterMovementComponent.SetGravityDirection` (`Character.CharacterMovement` `_as캐릭터`) (`KismetMathLibrary.GetDirectionUnitVector` (`self.K2_GetActorLocation` `_as캐릭터`) (`self.K2_GetActorLocation`)))
  (bind _asbp_gravity_character (cast `/Game/Asset/Gravity/BP_GravityCharacter` OtherActor))
  (set `/Game/Asset/Gravity/BP_GravityCharacter.AActor` OtherActor _asbp_gravity_character))

(event `self.ReceiveActorEndOverlap`
  (params (OtherActor :type "Actor Object Reference"))
  (bind _asbp_gravity_character (cast `/Game/Asset/Gravity/BP_GravityCharacter` OtherActor))
  (set `/Game/Asset/Gravity/BP_GravityCharacter.AActor` null _asbp_gravity_character))

(fn `UserConstructionScript`)